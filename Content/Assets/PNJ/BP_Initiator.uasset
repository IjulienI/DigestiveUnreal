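; BP_Initiator is an NPC that starts a dialog, or opens a merchant widget instead when flagged as a merchant.
; E_Dialog creates WBP_Dialogs once through a DoOnce and skips it on repeat calls while talking.
; Tick smoothly turns the NPC toward the passed position during dialog, then back to its initial rotation.
; E_ResetDialog ends the dialog, reveals the BP_Pointer hidden at BeginPlay, enables the HUD notification and re-arms the DoOnce.
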(event `self.ReceiveBeginPlay`
  (set `self.InitialRotation` (`self.K2_GetActorRotation`))
  (bind _returnvalue (`GameplayStatics.GetActorOfClass` "/Game/Game/Blueprints/Base/BP_Pointer.BP_Pointer_C"))
  (bind _output_get (set `self.Pointer` _returnvalue))
  (`self.SetActorHiddenInGame` _output_get true))

(event `self.ReceiveTick`
  (params (DeltaSeconds :type "Float (single-precision)"))
  (if (`self.InDialog`)
    (`self.K2_SetActorRotation` (`KismetMathLibrary.RLerp` (`self.K2_GetActorRotation`) (`KismetMathLibrary.FindLookAtRotation` (`self.K2_GetActorLocation`) (`self.TargetPosition`)) 0.2 true))
    (else
      (`self.K2_SetActorRotation` (`KismetMathLibrary.RLerp` (`self.K2_GetActorRotation`) (`self.InitialRotation`) 0.2 true)))))

(event `E_ResetDialog`
  (set `self.InDialog` false)
  (`self.SetActorHiddenInGame` (`self.Pointer`) false)
  (`/Game/Game/Blueprints/Widget/WBP_HUD.E_EnableNotif` (`self.HUD`))
  (goto _label :!via `Reset`))

(event `E_Dialog`
  (params (Position :type "Vector Structure") (HUD :type "/Game/Game/Blueprints/Widget/WBP_HUD Object Reference"))
  (if (not (`self.IsMerchand`))
    (set `self.HUD` HUD)
    (if (`self.InDialog`)
      (`/Game/Game/Blueprints/Widget/WBP_Dialogs.E_SkipDialog` (`self.DialogWidget`))
      (else
        (`/Engine/EditorBlueprintResources/StandardMacros.DoOnce` false :!label _label
          (:`Completed`
            (set `self.InDialog` true)
            (set `self.TargetPosition` Position)
            (bind _returnvalue (`|CreateWidget` "/Game/Game/Blueprints/Widget/WBP_Dialogs.WBP_Dialogs_C"))
            (bind _output_get (set `self.DialogWidget` _returnvalue))
            (`UserWidget.AddToViewport` _output_get 0)
            (`/Game/Game/Blueprints/Widget/WBP_Dialogs.E_StockInfo` (`self.DialogWidget`) self)))))
    (else
      (bind _returnvalue_2 (`|CreateWidget` "/Game/Game/Blueprints/Widget/WBP_Merchand.WBP_Merchand_C"))
      (`UserWidget.AddToViewport` _returnvalue_2 0))))

(fn `UserConstructionScript`)